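; Prototype boss hand actor that slams down on the player and can then be shot at a randomly chosen weak piece.
; On spawn, timelines slide it over the player, then after a delay lower it toward Z zero.
; Touching it during the attack deals massive damage; the landing damages non-falling players and reddens the weak piece.
; Projectile hits on that piece notify the boss and destroy the hand at a hit limit.
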(event OnComponentBeginOverlap(Collision)
  (params (OverlappedComponent :type Primitive%20Component%20Object%20Reference) (OtherActor :type Actor%20Object%20Reference) (OtherComp :type Primitive%20Component%20Object%20Reference) (OtherBodyIndex :type Integer) (bFromSweep :type Boolean) (SweepResult :type Hit%20Result%20Structure%20%28by%20ref%29))
  (if (== OtherActor (Variables|References|GetPlayerRef))
    (Utilities|FlowControl|DoOnce false
      (:Completed
        (Default|SetHealth (Variables|References|GetGI_Ref) -99.0)
        (Development|PrintString "YouGotHitGameOver" true true "(R=1.000000,G=0.019042,B=0.000000,A=1.000000)" 2.0 "Death")))))

(event OnComponentHit(Palm)
  (params (HitComponent :type Primitive%20Component%20Object%20Reference) (OtherActor :type Actor%20Object%20Reference) (OtherComp :type Primitive%20Component%20Object%20Reference) (NormalImpulse :type Vector :default "0, 0, 0") (Hit :type Hit%20Result%20Structure%20%28by%20ref%29))
  (CallFunction|PieceHit OtherActor HitComponent))

(event OnComponentHit(F1)
  (params (HitComponent :type Primitive%20Component%20Object%20Reference) (OtherActor :type Actor%20Object%20Reference) (OtherComp :type Primitive%20Component%20Object%20Reference) (NormalImpulse :type Vector :default "0, 0, 0") (Hit :type Hit%20Result%20Structure%20%28by%20ref%29))
  (CallFunction|PieceHit OtherActor HitComponent))

(event OnComponentHit(F2)
  (params (HitComponent :type Primitive%20Component%20Object%20Reference) (OtherActor :type Actor%20Object%20Reference) (OtherComp :type Primitive%20Component%20Object%20Reference) (NormalImpulse :type Vector :default "0, 0, 0") (Hit :type Hit%20Result%20Structure%20%28by%20ref%29))
  (CallFunction|PieceHit OtherActor HitComponent))

(event OnComponentHit(F3)
  (params (HitComponent :type Primitive%20Component%20Object%20Reference) (OtherActor :type Actor%20Object%20Reference) (OtherComp :type Primitive%20Component%20Object%20Reference) (NormalImpulse :type Vector :default "0, 0, 0") (Hit :type Hit%20Result%20Structure%20%28by%20ref%29))
  (CallFunction|PieceHit OtherActor HitComponent))

(event OnComponentHit(F4)
  (params (HitComponent :type Primitive%20Component%20Object%20Reference) (OtherActor :type Actor%20Object%20Reference) (OtherComp :type Primitive%20Component%20Object%20Reference) (NormalImpulse :type Vector :default "0, 0, 0") (Hit :type Hit%20Result%20Structure%20%28by%20ref%29))
  (CallFunction|PieceHit OtherActor HitComponent))

(event OnComponentHit(F5)
  (params (HitComponent :type Primitive%20Component%20Object%20Reference) (OtherActor :type Actor%20Object%20Reference) (OtherComp :type Primitive%20Component%20Object%20Reference) (NormalImpulse :type Vector :default "0, 0, 0") (Hit :type Hit%20Result%20Structure%20%28by%20ref%29))
  (CallFunction|PieceHit OtherActor HitComponent))

(event Custom|Decent
  (bind _returnvalue (Transformation|GetActorLocation))
  (Utilities|FlowControl|Delay 2.0)
  (bind _decenttrack (Timeline|DecendTimeline Play)
    (:Update
      (Transformation|SetActorLocation (Math|Vector|MakeVector (.x _returnvalue) (.y _returnvalue) (Math|Float|Lerp (.z _returnvalue) 0.0 _decenttrack)) true false))
    (:Finished
      (Development|PrintString "AOE Slam Activated ")
      (bind _output_get (Variables|Default|SetValurnableMesh (Utilities|Array|Get(acopy) (Utilities|Array|MakeArray (Variables|Meshes|GetPalm) (Variables|Meshes|GetF1) (Variables|Meshes|GetF2) (Variables|Meshes|GetF3) (Variables|Meshes|GetF4) (Variables|Meshes|GetF5)) (Math|Random|RandomIntegerinRange 0 5))))
      (Rendering|Material|SetMaterial _output_get 0 "/Game/LevelPrototyping/Materials/MI_Red.MI_Red")
      (CallFunction|DamageAOEifNotFalling)
      (Collision|SetCollisionEnabled (Variables|Default|GetCollision) "NoCollision"))))

(event EventBeginPlay
  (bind _returnvalue (Transformation|GetActorLocation))
  (bind _returnvalue_2 (Transformation|GetActorLocation))
  (bind _playerref (Variables|References|GetPlayerRef))
  (bind _returnvalue_3 (Transformation|GetActorLocation _playerref))
  (bind _asbp_gi (Utilities|Casting|CastToBP_GI (Game|GetGameInstance)))
  (Variables|References|SetGI_Ref _asbp_gi)
  (bind _newtrack_0 (Timeline|SetPositionOverPlayer Play)
    (:Update
      (Transformation|SetActorLocation (Math|Vector|Lerp(Vector) (Math|Vector|MakeVector (.x _returnvalue_2) (.y _returnvalue_2) (.z _returnvalue_2)) (Math|Vector|MakeVector (.x _returnvalue_3) (.y _returnvalue_3) (.z _returnvalue_2)) _newtrack_0) true false)
      (bind _outhit (Collision|LineTraceByChannel (Transformation|GetActorLocation) (Math|Vector|MakeVector (.x _returnvalue) (.y _returnvalue) 0.0) "TraceTypeQuery1" false 0 "ForDuration"))
      (Variables|Default|SetHandDestinationHeight (.Z (Math|Vector|BreakVector (.ImpactPoint (Collision|BreakHitResult _outhit))))))
    (:Finished
      (CallFunction|Decent))))

(fn ConstructionScript)

(fn DamageAOEifNotFalling
  (bind _isfalling (Class|BPIPlayer|GetIsFalling(Message) (Variables|References|GetPlayerRef)))
  (if (not _isfalling)
    (Default|SetHealth (Variables|References|GetGI_Ref) -2e+01)
    (Collision|SetCollisionEnabled (Variables|Default|GetCollision) "NoCollision")))

(fn PieceHit
  (params (HittingActor :type Actor%20Object%20Reference) (HitComponent :type Object%20Object%20Reference))
  (if (Class|GameplayStatics|ObjectIsA HittingActor "/Game/Variant_Shooter/Blueprints/Pickups/Projectiles/BP_FirstPersonProjectile.BP_FirstPersonProjectile_C")
    (if (== HitComponent (Variables|Default|GetValurnableMesh))
      (Development|PrintString "ValurnableMeshHit")
      (bind _result (Math|Integer|IncrementInt (Variables|Default|GetTimesHit))
        (:%20%20
          (Class|BPIBoss|GetHit(Message) (Variables|References|GetBossRef))
          (if (== _result (Variables|Default|GetMaxHitsPerComponent))
            (Rendering|SetActorHiddenInGame true)
            (Transformation|SetActorLocation "0.000000,0.000000,-555.000000" false true)
            (Actor|DestroyActor))))
      (else
        (Development|PrintString "INValurnableMeshHit")))))