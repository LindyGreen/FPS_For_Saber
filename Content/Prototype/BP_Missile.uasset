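; Prototype homing missile that seeks the player's "Homing"-tagged component and damages them through health stored in the BP_GI game instance.
; Overlapping the player counts as a direct hit, playing a 2D sound and dealing heavy damage.
; Any other overlap plays a located explosion and runs a debug-drawn sphere trace for lighter splash damage to the player.
; Both impacts destroy the missile, with print strings standing in for VFX.
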(event OnComponentBeginOverlap(Sphere)
  (params (OverlappedComponent :type Primitive%20Component%20Object%20Reference) (OtherActor :type Actor%20Object%20Reference) (OtherComp :type Primitive%20Component%20Object%20Reference) (OtherBodyIndex :type Integer) (bFromSweep :type Boolean) (SweepResult :type Hit%20Result%20Structure%20%28by%20ref%29))
  (bind _returnvalue (Transformation|GetActorLocation))
  (if (not (== OtherActor self))
    (if (== OtherActor (Variables|Default|GetPlayerRef))
      (Development|PrintString "ExplosionVFXOnPlayer")
      (Audio|PlaySound2D "/Game/Prototype/Audio/ExplosionSound.ExplosionSound" 1.0 1.0 0.0 0 0)
      ;[0.15 0.15 0.15 0.5] Direct Hit
      (Default|SetHealth (Variables|Default|GetGI_ref) -4e+01)
      (Actor|DestroyActor)
      (else
        (Development|PrintString "ExplosionVFXOnTheGround")
        (Audio|PlaySoundatLocation "/Game/Prototype/Audio/ExplosionSound.ExplosionSound" _returnvalue "0, 0, 0" 1.0 1.0 0.0 0 0 0 0)
        (bind _outhits (Collision|MultiSphereTraceByChannel _returnvalue _returnvalue 3e+02 "TraceTypeQuery1" false 0 "ForDuration" true "(R=1.000000,G=0.000000,B=0.000000,A=1.000000)" "(R=0.000000,G=1.000000,B=0.000000,A=1.000000)" 3.0))
        (for _array_element _outhits
          (if (== (.HitActor (Collision|BreakHitResult _array_element)) (Variables|Default|GetPlayerRef))
            (Default|SetHealth (Variables|Default|GetGI_ref) -2e+01)))
        (Actor|DestroyActor)))))

(event EventBeginPlay
  (Variables|/Script/Engine.ProjectileMovementComponent|SetHomingTargetComponent (Variables|Default|GetProjectileMovement) (Class|Actor|FindComponentbyTag (Variables|Default|GetPlayerRef) "/Script/Engine.SceneComponent" "Homing"))
  (bind _asbp_gi (Utilities|Casting|CastToBP_GI (Game|GetGameInstance)))
  (Variables|Default|SetGI_ref _asbp_gi))

(fn ConstructionScript)