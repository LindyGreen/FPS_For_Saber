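; BP_Lootbox is a prototype lootbox that rolls for rare or common loot whenever a BP_PistolBullet hits its Hitbox.
; The roll and running statistics come from LootMathGenerator.
; Results appear only as keyed on-screen debug prints, green for rare and red for common, followed by a rare-to-loot statistics line; no item is spawned.
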(event OnComponentHit(Hitbox)
  (params (HitComponent :type Primitive%20Component%20Object%20Reference) (OtherActor :type Actor%20Object%20Reference) (OtherComp :type Primitive%20Component%20Object%20Reference) (NormalImpulse :type Vector :default "0, 0, 0") (Hit :type Hit%20Result%20Structure%20%28by%20ref%29))
  (bind _lootmathgenerator (Variables|Default|GetLootMathGenerator))
  (if (Class|GameplayStatics|ObjectIsA OtherActor "/Game/Variant_Shooter/Blueprints/Pickups/Projectiles/BP_PistolBullet.BP_PistolBullet_C")
    (bind _output_get (Variables|Default|SetRareLoot (Class|LootMathGenerator|IsLootRare _lootmathgenerator)))
    (if _output_get
      (Development|PrintString "RareLoot" true true "(R=0.000698,G=0.338542,B=0.034549,A=1.000000)" 3.0 "Loot")
      (else
        (Development|PrintString "CommonLoot" true true "(R=1.000000,G=0.000000,B=0.000000,A=1.000000)" 3.0 "Loot")))
    (Development|PrintString (Utilities|String|Append "RareLoot/Loot" (Utilities|String|ToString(Float) (Class|LootMathGenerator|GetLootStatistics _lootmathgenerator))) true true "(R=0.000000,G=0.660000,B=1.000000,A=1.000000)" 2.0 "Loot2")))

(event EventBeginPlay)

(fn ConstructionScript)