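; Prototype boss that cycles on timers through Idle, Shooting and Slamming states, starting in Idle.
; OnBossStateBegin sets material color, warning sound and duration per state, and OnBossStateEnd picks the next.
; Shooting runs a looping timer that spawns BP_Missile actors carrying the player reference.
; Slamming has only color, sound and duration; the BP_hand spawn event is never called here.
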(event Custom|EventStopShooting
  (Utilities|Time|ClearTimerbyFunctionName 0 "ShootAMissile"))

(event Custom|EventChangeState
  (params (Timer :type Float%20%28double-precision%29))
  (Utilities|Time|SetTimerbyFunctionName 0 "OnBossStateEnd" Timer))

(event Custom|EventStartShooting
  (Utilities|Time|SetTimerbyFunctionName 0 "ShootAMissile" 2.0 true))

(event Custom|EventStartHandSpawn
  (Game|SpawnActorfromClass "/Game/Prototype/BP_hand.BP_hand_C" (Transformation|GetWorldTransform (Variables|Default|GetMissile%20Spawn%20point)) "Undefined" "MultiplyWithRoot" 0 0))

(event EventBeginPlay
  (Variables|Default|SetPlayerRef (Game|GetPlayerCharacter 0))
  (CallFunction|OnBossStateBegin "NewEnumerator0"))

(event Collision|EventActorBeginOverlap
  (params (OtherActor :type Actor%20Object%20Reference)))

(event EventTick
  (params (DeltaSeconds :type Float%20%28single-precision%29)))

(fn ConstructionScript)

(fn OnBossStateBegin
  (params (NewState :type E_BossStates%20Enum :default "NewEnumerator0"))
  (bind _output_get (Variables|Default|SetCurrentState NewState))
  (Rendering|Material|SetMaterial (Variables|Default|GetCube) 0 (Utilities|Select :Index _output_get :NewEnumerator0 "/Game/LevelPrototyping/Materials/MI_DefaultColorway.MI_DefaultColorway" :NewEnumerator1 "/Game/LevelPrototyping/Materials/MI_Red.MI_Red" :NewEnumerator2 "/Game/LevelPrototyping/Materials/MI_Orange.MI_Orange"))
  (Audio|PlaySound2D (Utilities|Select :Index _output_get :NewEnumerator0 0 :NewEnumerator1 "/Game/Prototype/Audio/SpankingIncoming.SpankingIncoming" :NewEnumerator2 "/Game/Prototype/Audio/MissilesIncoming.MissilesIncoming") 1.0 1.0 0.0 0 0)
  (CallFunction|EventChangeState (Utilities|Select :Index (Variables|Default|GetCurrentState) :NewEnumerator0 3.0 :NewEnumerator1 5.0 :NewEnumerator2 12.0))
  (switch Utilities|FlowControl|Switch|SwitchonE_BossStates (Variables|Default|GetCurrentState)
    (:NewEnumerator2
      (CallFunction|EventStartShooting))))

(fn OnBossStateEnd
  (switch Utilities|FlowControl|Switch|SwitchonE_BossStates (Variables|Default|GetCurrentState)
    (:NewEnumerator0
      (CallFunction|OnBossStateBegin (Utilities|Select :Index (Variables|Default|GetCurrentState) :NewEnumerator0 "NewEnumerator2" :NewEnumerator1 "NewEnumerator0" :NewEnumerator2 "NewEnumerator1") :!label _label))
    (:NewEnumerator1
      (goto _label))
    (:NewEnumerator2
      (Utilities|FlowControl|Sequence
        (:then_0
          (CallFunction|EventStopShooting))
        (:then_1
          (goto _label))))))

(fn ShootAMissile
  (Game|SpawnActorfromClass "/Game/Prototype/BP_Missile.BP_Missile_C" (Transformation|GetWorldTransform (Variables|Default|GetMissile%20Spawn%20point)) "Undefined" "MultiplyWithRoot" 0 (Variables|Default|GetPlayerRef) 0))