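; Prototype giant hand attack that, on BeginPlay, tracks over the player and slaps down.
; Two chained timelines lerp it horizontally with a debug trace, then vertically with sweep.
; Overlapping the player applies heavy health damage through BP_GI and prints game over.
; After landing, it damages a non-falling player regardless of distance and disables collision, then paints a random palm or finger mesh red as the apparent weak point.
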(event OnComponentBeginOverlap(Collision)
  (params (OverlappedComponent :type Primitive%20Component%20Object%20Reference) (OtherActor :type Actor%20Object%20Reference) (OtherComp :type Primitive%20Component%20Object%20Reference) (OtherBodyIndex :type Integer) (bFromSweep :type Boolean) (SweepResult :type Hit%20Result%20Structure%20%28by%20ref%29))
  (if (== OtherActor (Variables|Default|GetPlayerRef))
    (Default|SetHealth (Variables|Default|GetGI_Ref) -99.0)
    (Development|PrintString "YouGotHitGameOver")))

(event EventBeginPlay
  (bind _returnvalue (Transformation|GetActorLocation))
  (bind _returnvalue_2 (Transformation|GetActorLocation))
  (bind _playerref (Variables|Default|GetPlayerRef))
  (bind _returnvalue_3 (Transformation|GetActorLocation _playerref))
  (bind _asbp_gi (Utilities|Casting|CastToBP_GI (Game|GetGameInstance)))
  (Variables|Default|SetGI_Ref _asbp_gi)
  (bind _newtrack_0 (Timeline|SetPositionOverPlayer Play)
    (:Update
      (Transformation|SetActorLocation (Math|Vector|Lerp(Vector) (Math|Vector|MakeVector (.x _returnvalue_2) (.y _returnvalue_2) (.z _returnvalue_2)) (Math|Vector|MakeVector (.x _returnvalue_3) (.y _returnvalue_3) (.z _returnvalue_2)) _newtrack_0) false false)
      (Collision|LineTraceByChannel (Transformation|GetActorLocation) (Math|Vector|MakeVector (.x _returnvalue) (.y _returnvalue) 0.0) "TraceTypeQuery1" false 0 "ForDuration"))
    (:Finished
      (bind _newtrack_0_2 (Timeline|SlapTileline Play)
        (:Update
          (Transformation|SetActorLocation (Math|Vector|Lerp(Vector) (Math|Vector|MakeVector (.x _returnvalue_2) (.y _returnvalue_2) (.z _returnvalue_2)) (Math|Vector|MakeVector (.x _returnvalue_2) (.y _returnvalue_2) (.z _returnvalue_3)) _newtrack_0_2) true false))
        (:Finished
          (CallFunction|DamageAOEifNotFalling)
          (bind _output_get (Variables|Default|SetValurnableMesh (Utilities|Array|Get(acopy) (Utilities|Array|MakeArray (Variables|Meshes|GetCube) (Variables|Meshes|GetF1) (Variables|Meshes|GetF2) (Variables|Meshes|GetF3) (Variables|Meshes|GetF4) (Variables|Meshes|GetF5)) (Math|Random|RandomIntegerinRange 0 5))))
          (Rendering|Material|SetMaterial _output_get 0 "/Game/LevelPrototyping/Materials/MI_Red.MI_Red"))))))

(fn ConstructionScript)

(fn DamageAOEifNotFalling
  (bind _isfalling (Class|BPIPlayer|GetIsFalling(Message) (Variables|Default|GetPlayerRef)))
  (if (not _isfalling)
    (Default|SetHealth (Variables|Default|GetGI_Ref) -2e+01)
    (Collision|SetCollisionEnabled (Variables|Default|GetCollision) "NoCollision")))